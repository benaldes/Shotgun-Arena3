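; Air launcher weapon that knocks the player backward and blasts enemies away along the first-person camera's aim.
; Fire launches the player against the view direction with damped vertical recoil and a small lift, then plays rocket launcher animation and sound.
; A short forward sphere trace on pawns gives each BP_EnemyAI hit a small hop, then a delayed forward-and-up launch, using a Delay inside the loop.
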(event EventBeginPlay
  (|CallParentFunction) ; This node is disabled and will not be called.\nDrag off pins to build functionality.
)

(event Collision|EventActorBeginOverlap
  (params (OtherActor :type Actor%20Object%20Reference))
  (|CallParentFunction OtherActor) ; This node is disabled and will not be called.\nDrag off pins to build functionality.
)

(event EventTick
  (params (DeltaSeconds :type Float%20%28single-precision%29))
  (|CallParentFunction DeltaSeconds) ; This node is disabled and will not be called.\nDrag off pins to build functionality.
)

(event EventFire
  (bind _returnvalue (Game|GetPlayerCharacter 0))
  (bind _asbp_first_person_character (Utilities|Casting|CastToBP_FirstPersonCharacter _returnvalue))
  (Character|LaunchCharacter _returnvalue (Math|Vector|MakeVector (* (.x (* (Math|Vector|GetForwardVector (Transformation|GetWorldRotation (Variables|/Game/FirstPerson/Blueprints/BP_FirstPersonCharacter.BP_FirstPersonCharacter_C|GetFirstPersonCamera _asbp_first_person_character))) 1500)) -1.0) (* (.y (* (Math|Vector|GetForwardVector (Transformation|GetWorldRotation (Variables|/Game/FirstPerson/Blueprints/BP_FirstPersonCharacter.BP_FirstPersonCharacter_C|GetFirstPersonCamera _asbp_first_person_character))) 1500)) -1.0) (+ (* (.z (* (Math|Vector|GetForwardVector (Transformation|GetWorldRotation (Variables|/Game/FirstPerson/Blueprints/BP_FirstPersonCharacter.BP_FirstPersonCharacter_C|GetFirstPersonCamera _asbp_first_person_character))) 1500)) -0.3) 1.5e+02)) false false)
  (Components|Animation|PlayAnimation (Variables|Default|GetWeaponModel) "/Game/MilitaryWeapDark/Weapons/Anims/Fire_RocketLauncher_W.Fire_RocketLauncher_W" false)
  (Audio|PlaySound2D "/Game/MilitaryWeapDark/Sound/RocketLauncher/wavs/RocketLauncher_Explosion01.RocketLauncher_Explosion01" 1.0 1.0 0.0 0 0)
  (bind _asbp_first_person_character_2 (Utilities|Casting|CastToBP_FirstPersonCharacter (Game|GetPlayerCharacter 0)))
  (bind _outhits (Collision|MultiSphereTraceForObjects (Transformation|GetWorldLocation (Variables|/Game/FirstPerson/Blueprints/BP_FirstPersonCharacter.BP_FirstPersonCharacter_C|GetFirstPersonCamera _asbp_first_person_character_2)) (+ (Transformation|GetWorldLocation (Variables|/Game/FirstPerson/Blueprints/BP_FirstPersonCharacter.BP_FirstPersonCharacter_C|GetFirstPersonCamera _asbp_first_person_character_2)) (* (Math|Vector|GetForwardVector (Transformation|GetWorldRotation (Variables|/Game/FirstPerson/Blueprints/BP_FirstPersonCharacter.BP_FirstPersonCharacter_C|GetFirstPersonCamera _asbp_first_person_character_2))) 6e+02)) 1e+02 (Utilities|Array|MakeArray "ObjectTypeQuery3") false (Utilities|Array|MakeArray (Game|GetPlayerCharacter 0)) "None"))
  (bind _array_element (Utilities|Array|ForEachLoopwithBreak _outhits)
    (:LoopBody
      (bind _asbp_enemy_ai (Utilities|Casting|CastToBP_EnemyAI (.HitActor (Collision|BreakHitResult _array_element))))
      (Character|LaunchCharacter _asbp_enemy_ai (Math|Vector|MakeVector 0.0 0.0 1e+02) false false)
      (Utilities|FlowControl|Delay 0.1)
      (Character|LaunchCharacter _asbp_enemy_ai (Math|Vector|MakeVector (.x (* (Math|Vector|GetForwardVector (Transformation|GetWorldRotation (Variables|/Game/FirstPerson/Blueprints/BP_FirstPersonCharacter.BP_FirstPersonCharacter_C|GetFirstPersonCamera _asbp_first_person_character_2))) 1500)) (.y (* (Math|Vector|GetForwardVector (Transformation|GetWorldRotation (Variables|/Game/FirstPerson/Blueprints/BP_FirstPersonCharacter.BP_FirstPersonCharacter_C|GetFirstPersonCamera _asbp_first_person_character_2))) 1500)) (+ (.z (* (Math|Vector|GetForwardVector (Transformation|GetWorldRotation (Variables|/Game/FirstPerson/Blueprints/BP_FirstPersonCharacter.BP_FirstPersonCharacter_C|GetFirstPersonCamera _asbp_first_person_character_2))) 1500)) 5e+02)) false false))))

(fn ConstructionScript
  (|CallParentFunction))