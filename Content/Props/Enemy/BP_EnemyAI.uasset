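; Zombie enemy Blueprint that chases the player once spotted, attacks in melee and dies when its HP runs out.
; PawnSensing starts an AI MoveTo loop that plays the attack animation, then damages the player after a delay if IsPlayerInRange is still set.
; HitDetect overlaps set that flag without filtering for the player.
; ReciveDamage lowers HP and, on death, plays sound and animation, stops movement and disables collision.
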(event OnSeePawn(PawnSensing)
  (params (Pawn :type Pawn%20Object%20Reference))
  (if (not (Variables|Default|GetIsDead?))
    (Variables|Default|SetIsSeeingPlayer true)
    (CallFunction|FollowPlayer)))

(event OnComponentBeginOverlap(HitDetect)
  (params (OverlappedComponent :type Primitive%20Component%20Object%20Reference) (OtherActor :type Actor%20Object%20Reference) (OtherComp :type Primitive%20Component%20Object%20Reference) (OtherBodyIndex :type Integer) (bFromSweep :type Boolean) (SweepResult :type Hit%20Result%20Structure%20%28by%20ref%29))
  (if (not (Variables|Default|GetIsDead?))
    (Variables|Default|SetIs%20Player%20In%20Range? true)))

(event OnComponentEndOverlap(HitDetect)
  (params (OverlappedComponent :type Primitive%20Component%20Object%20Reference) (OtherActor :type Actor%20Object%20Reference) (OtherComp :type Primitive%20Component%20Object%20Reference) (OtherBodyIndex :type Integer))
  (if (not (Variables|Default|GetIsDead?))
    (Variables|Default|SetIs%20Player%20In%20Range? false)))

(event Custom|FollowPlayer
  (if (not (Variables|Default|GetIsDead?)) :!label _label
    (if (Variables|Default|GetisNotAttacking)
      (if (Variables|Default|GetIsSeeingPlayer)
        (AI|AIMoveTo self "0, 0, 0" (Game|GetPlayerCharacter 0) 7e+01 false
          (:OnSuccess
            (if (Variables|Default|GetcanAttack?)
              (Variables|Default|SetcanAttack? false)
              (Variables|Default|SetisNotAttacking false)
              (Components|Animation|PlayAnimation (Variables|Character|GetMesh) "/Game/Props/Enemy/animation/Zombie_Attack.Zombie_Attack" false)
              (Utilities|FlowControl|Delay 1.4)
              (if (not (Variables|Default|GetIsDead?))
                (if (Variables|Default|GetIs%20Player%20In%20Range?)
                  (bind _asbp_first_person_character (Utilities|Casting|CastToBP_FirstPersonCharacter (Game|GetPlayerCharacter 0)))
                  (Default|ReciveDamage _asbp_first_person_character))
                (Utilities|FlowControl|Delay 1.4)
                (Variables|Default|SetcanAttack? true)
                (Variables|Default|SetisNotAttacking true)
                (Class|SkeletalMeshComponent|SetAnimClass (Variables|Character|GetMesh) "/Game/Props/Enemy/AP_ZombieAI.AP_ZombieAI_C")
                (goto _label)))))))))

(event Custom|ReciveDamage
  (params (DMG :type Integer))
  (if (not (Variables|Default|GetIsDead?))
    (Audio|PlaySound2D "/Game/Sound/Something_being_hit_-_Sound_Effect.Something_being_hit_-_Sound_Effect" 1.0 1.0 0.0 0 0)
    (Variables|Default|SetHP (- (Variables|Default|GetHP) DMG))
    (if (<= (Variables|Default|GetHP) 0)
      (Audio|PlaySound2D "/Game/Sound/Die_Sound_Effect.Die_Sound_Effect" 1.0 1.0 0.0 0 0)
      (Components|Animation|PlayAnimation (Variables|Character|GetMesh) "/Game/Props/Enemy/animation/zombie_dying.zombie_dying" false)
      (Variables|Default|SetIsDead? true)
      (Components|Movement|StopMovementImmediately (Variables|Character|GetCharacterMovement))
      (Collision|SetActorEnableCollision false))))

(event EventBeginPlay)

(event Collision|EventActorBeginOverlap
  (params (OtherActor :type Actor%20Object%20Reference)))

(event EventTick
  (params (DeltaSeconds :type Float%20%28single-precision%29)))

(fn ConstructionScript)