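; BP_WeaponPickUp is a world pickup that gives a weapon and its ammo to the interacting character.
; Interact passes the weapon, ammo data and pickup location to the character's SpawnWeapon, plays a sound and destroys the actor.
; Functions also expose the ammo struct and let reserve ammo be taken without collecting the weapon, subtracting it and popping the object upward with a randomized impulse and sound.
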(event EventBeginPlay
  (|CallParentFunction) ; This node is disabled and will not be called.\nDrag off pins to build functionality.
)

(event Collision|EventActorBeginOverlap
  (params (OtherActor :type Actor%20Object%20Reference))
  (|CallParentFunction OtherActor) ; This node is disabled and will not be called.\nDrag off pins to build functionality.
)

(event EventTick
  (params (DeltaSeconds :type Float%20%28single-precision%29))
  (|CallParentFunction DeltaSeconds) ; This node is disabled and will not be called.\nDrag off pins to build functionality.
)

(event EventInteract
  (params (CharacterPickUp :type BP%20First%20Person%20Character%20Object%20Reference))
  (Default|SpawnWeapon CharacterPickUp (Variables|Default|GetWeaponToSpawn) (Transformation|GetActorLocation) (Variables|Default|GetAmmo) (Variables|Default|GetAmmo%20Type))
  (Audio|PlaySound2D "/Game/MilitaryWeapDark/Sound/Pistol/Pistol_AmmoPickup_Cue.Pistol_AmmoPickup_Cue" 1.0 1.0 0.0 0 0)
  (Actor|DestroyActor))

(event EventIFTakeReserveAmmo
  (params (AmmoTaken :type Integer))
  (if (> (.ResorveAmmo (Utilities|Struct|BreakStruct_Ammo (Variables|Default|GetAmmo%20Type))) 0)
    (Variables|Default|SetAmmo%20Type (Utilities|Struct|MakeStruct_Ammo (.AmmoType (Utilities|Struct|BreakStruct_Ammo (Variables|Default|GetAmmo%20Type))) (.AmmoIndex (Utilities|Struct|BreakStruct_Ammo (Variables|Default|GetAmmo%20Type))) (- (.ResorveAmmo (Utilities|Struct|BreakStruct_Ammo (Variables|Default|GetAmmo%20Type))) AmmoTaken) (.MaxResorveAmmo (Utilities|Struct|BreakStruct_Ammo (Variables|Default|GetAmmo%20Type))) (.Has? (Utilities|Struct|BreakStruct_Ammo (Variables|Default|GetAmmo%20Type)))))
    (Physics|AddImpulse (Variables|Default|GetPickUpObject) (Math|Vector|MakeVector (Math|Random|RandomFloatinRange -25.0 25.0) (Math|Random|RandomFloatinRange -25.0 25.0) (Math|Random|RandomFloatinRange 125.0 1.5e+02)) "None" false)
    (Audio|PlaySoundatLocation "/Game/MilitaryWeapDark/Sound/Pistol/Wavs/Pistol_AmmoPickup.Pistol_AmmoPickup" (Transformation|GetActorLocation) "0, 0, 0" 1.0 1.0 0.0 0 0 0 0)))

(fn ConstructionScript
  (|CallParentFunction))

(fn IFGetAmmoType
  (return (Variables|Default|GetAmmo%20Type)))